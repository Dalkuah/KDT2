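; BP_HelloActor is a test-style actor that shuttles its Sphere component back and forth along world X while spinning it.
; Tick offsets the sphere by Speed scaled with delta time, while the spin is a fixed step per frame.
; IsMoveRight selects the direction and flips at hard-coded X limits, along with a half-turn world rotation.
; Disconnected print-loop and relative-location nodes never run.
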(event EventTick
  (params (DeltaSeconds :type Float%20%28single-precision%29))
  (bind _sphere (Variables|Default|GetSphere))
  (bind _sphere_2 (Variables|Default|GetSphere))
  (if (Variables|Default|GetIsMoveRight)
    ;[0 1 0.6541] 오른쪽으로 이동
    (Transformation|AddWorldOffset _sphere (Math|Vector|MakeVector (* DeltaSeconds (Variables|Default|GetSpeed)) 0.0 0.0) false false)
    (Transformation|AddRelativeRotation _sphere "0.000000,10.000000,0.000000" false false)
    (if (>= (.x (Transformation|GetWorldLocation _sphere)) 1e+04)
      (Transformation|AddWorldRotation _sphere "0.000000,180.000000,0.000000" false false)
      (Variables|Default|SetIsMoveRight false))
    (else
      ;[0.2113 0 1 1 20] 왼쪽으로 이동
      (Transformation|AddWorldOffset _sphere_2 (Math|Vector|MakeVector (* (* DeltaSeconds (Variables|Default|GetSpeed)) -1.0) 0.0 0.0) false false)
      (Transformation|AddRelativeRotation _sphere_2 "0.000000,10.000000,0.000000" false false)
      (if (< (.x (Transformation|GetWorldLocation _sphere_2)) -1e+04)
        (Transformation|AddWorldRotation _sphere_2 "0.000000,180.000000,0.000000" false false)
        (Variables|Default|SetIsMoveRight true)))))

(event EventBeginPlay)

(fn ConstructionScript)