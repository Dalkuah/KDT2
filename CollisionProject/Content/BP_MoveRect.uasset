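; BP_MoveRect is an actor that moves its Cube component around a rectangular loop in the local XZ plane while play is enabled.
; Tick switches on the SetMove state, shifting the cube by Speed times delta time and advancing to the next direction at each 0 or 500 bound, cycling right, up, left and down.
; EventPlay and EventStop toggle IsPlay, and Tick also accumulates elapsed time in TotalSec while playing.
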(event EventEventStop
  (Variables|Default|SetIsPlay false))

(event EventEventPlay
  (Variables|Default|SetIsPlay true))

(event EventTick
  (params (DeltaSeconds :type Float%20%28single-precision%29))
  (bind _cube (Variables|Default|GetCube))
  (bind _cube_2 (Variables|Default|GetCube))
  (bind _cube_3 (Variables|Default|GetCube))
  (bind _cube_4 (Variables|Default|GetCube))
  (if (Variables|Default|GetIsPlay)
    (Variables|Default|SetTotalSec (+ DeltaSeconds (Variables|Default|GetTotalSec)))
    (switch Utilities|FlowControl|Switch|SwitchonMove (Variables|Default|GetsetMove)
      (:NewEnumerator0
        ;[0.06128 0 1] 오른쪽으로 이동
        (Transformation|AddRelativeLocation _cube_2 (Math|Vector|MakeVector (* DeltaSeconds (Variables|Default|GetSpeed)) 0.0 0.0) false false)
        (if (>= (.x (Variables|/Script/Engine.SceneComponent|GetRelativeLocation _cube_2)) 5e+02)
          (Variables|Default|SetsetMove "NewEnumerator1")))
      (:NewEnumerator1
        (Transformation|AddRelativeLocation _cube_4 (Math|Vector|MakeVector 0.0 0.0 (* DeltaSeconds (Variables|Default|GetSpeed))) false false)
        (if (>= (.z (Variables|/Script/Engine.SceneComponent|GetRelativeLocation _cube_4)) 5e+02)
          (Variables|Default|SetsetMove "NewEnumerator2")))
      (:NewEnumerator2
        ;[0 1 0.883] 왼쪽으로 이동
        (Transformation|AddRelativeLocation _cube_3 (Math|Vector|MakeVector (* (* DeltaSeconds (Variables|Default|GetSpeed)) -1.0) 0.0 0.0) false false)
        (if (< (.x (Variables|/Script/Engine.SceneComponent|GetRelativeLocation _cube_3)) 0.0)
          (Variables|Default|SetsetMove "NewEnumerator3")))
      (:NewEnumerator3
        (Transformation|AddRelativeLocation _cube (Math|Vector|MakeVector 0.0 0.0 (* (* DeltaSeconds (Variables|Default|GetSpeed)) -1.0)) false false)
        (if (< (.z (Variables|/Script/Engine.SceneComponent|GetRelativeLocation _cube)) 0.0)
          (Variables|Default|SetsetMove "NewEnumerator0"))))))

(fn ConstructionScript)