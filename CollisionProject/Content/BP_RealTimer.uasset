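; BP_RealTimer is an in-world stopwatch that accumulates time while something overlaps its Cube component and pauses when an overlap ends.
; Overlap begin and end set IsPlay, which lets Tick add delta seconds to a running total that is never reset.
; While running, TextRender shows red MM:SS text zero-padded by STR00, and it turns grey when paused.
; The START and STOP events are empty, with their IsPlay setters left unconnected.
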(event OnComponentBeginOverlap(Cube)
  (params (OverlappedComponent :type Primitive%20Component%20Object%20Reference) (OtherActor :type Actor%20Object%20Reference) (OtherComp :type Primitive%20Component%20Object%20Reference) (OtherBodyIndex :type Integer) (bFromSweep :type Boolean) (SweepResult :type Hit%20Result%20Structure%20%28by%20ref%29))
  (Variables|Default|SetIsPlay true))

(event OnComponentEndOverlap(Cube)
  (params (OverlappedComponent :type Primitive%20Component%20Object%20Reference) (OtherActor :type Actor%20Object%20Reference) (OtherComp :type Primitive%20Component%20Object%20Reference) (OtherBodyIndex :type Integer))
  (Variables|Default|SetIsPlay false))

(event EventTick
  (params (DeltaSeconds :type Float%20%28single-precision%29))
  (bind _returnvalue (Math|Color|MakeColor 1.0 1.0 1.0))
  (bind _textrender (Variables|Default|GetTextRender))
  (if (Variables|Default|GetIsPlay)
    (bind _output_get (Variables|Default|SetTotalSec (+ DeltaSeconds (Variables|Default|GetTotalSec))))
    (Rendering|Components|TextRender|SetText _textrender (Utilities|Text|ToText(String) (Utilities|String|Append (CallFunction|STR00 (/ _output_get 6e+01)) ":" (CallFunction|STR00 (Math|Float|%(Float) _output_get 6e+01)))))
    (Rendering|Components|TextRender|SetTextRenderColor _textrender (Math|Conversions|ToColor(LinearColor) (* _returnvalue "(R=1.000000,G=0.000000,B=0.000000,A=1.000000)")))
    (else
      (Rendering|Components|TextRender|SetTextRenderColor _textrender (Math|Conversions|ToColor(LinearColor) (* _returnvalue "(R=0.500000,G=0.500000,B=0.500000,A=1.000000)"))))))

(event EventSTOP)

(event EventSTART)

(fn ConstructionScript)

(fn STR00
  (params (Num :type Float%20%28double-precision%29))
  (bind _returnvalue (Math|Float|Floor Num))
  (bind _returnvalue_2 (Utilities|String|ToString(Integer) _returnvalue))
  (if (< _returnvalue 10)
    (return (Utilities|String|Append "0" _returnvalue_2))
    (else
      (return _returnvalue_2))))