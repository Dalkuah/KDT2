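; BP_Homing is a homing hazard that chases the first player character and ragdolls it on contact.
; Tick moves it a fixed step per frame along its Arrow, without delta scaling or sweep, while RInterpTo gradually turns it toward the target.
; A Sphere overlap with BP_ThirdPersonCharacter triggers the ragdoll, destroys the actor and spawns an explosion.
; Otherwise, it self-destructs with an effect after a delay started in BeginPlay.
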(event OnComponentBeginOverlap(Sphere)
  (params (OverlappedComponent :type Primitive%20Component%20Object%20Reference) (OtherActor :type Actor%20Object%20Reference) (OtherComp :type Primitive%20Component%20Object%20Reference) (OtherBodyIndex :type Integer) (bFromSweep :type Boolean) (SweepResult :type Hit%20Result%20Structure%20%28by%20ref%29))
  (bind _returnvalue (Transformation|GetActorTransform))
  (bind _asbp_third_person_character (Utilities|Casting|CastToBP_ThirdPersonCharacter OtherActor))
  (Default|DoRagdoll _asbp_third_person_character)
  (Actor|DestroyActor)
  (Effects|SpawnEmitteratLocation "/Game/StarterContent/Particles/P_Explosion.P_Explosion" (.location _returnvalue) (.rotation _returnvalue) "2.000000,2.000000,2.000000"))

(event Custom|TimeOver
  (Niagara|SpawnSystematLocation "/Game/CoinGame/Good.Good" (Transformation|GetActorLocation))
  (Components|Activation|SetActive (Variables|Default|GetDeathFx) true false)
  (Actor|DestroyActor))

(event EventTick
  (params (DeltaSeconds :type Float%20%28single-precision%29))
  (Utilities|IsValid (Variables|Default|GetHomingTarget)
    (:Is%20Valid
      (Transformation|AddActorWorldOffset (* (Math|Vector|GetForwardVector (Variables|Default|GetArrow)) 8.0))
      (Transformation|SetActorRotation (Math|Interpolation|RInterpTo (Transformation|GetActorRotation) (Math|Rotator|FindLookatRotation (Transformation|GetActorLocation) (Transformation|GetActorLocation (Variables|Default|GetHomingTarget))) DeltaSeconds 2.0)))))

(event EventBeginPlay
  (Variables|Default|SetHomingTarget (Game|GetPlayerCharacter 0))
  (Utilities|FlowControl|Delay 1e+01)
  (CallFunction|TimeOver))

(fn ConstructionScript)