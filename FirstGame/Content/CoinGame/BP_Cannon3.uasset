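; BP_Cannon3 is a cannon actor in CoinGame that rapidly fires bullets along a fixed direction.
; On BeginPlay it stores the player character as Target and starts a fast looping timer that calls ShootBullet.
; ShootBullet spawns a BP_Bullet at the Arrow component's world transform.
; Smoothed look-at rotation toward the player exists in the graph but is disconnected, so the cannon does not track.
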(event EventBeginPlay
  (Variables|Default|SetTarget (Game|GetPlayerCharacter 0))
  (Utilities|Time|SetTimerbyFunctionName 0 "ShootBullet" 0.05 true))

(event EventTick
  (params (DeltaSeconds :type Float%20%28single-precision%29)))

(fn ConstructionScript)

(fn ShootBullet
  (Game|SpawnActorfromClass "/Game/CoinGame/BP_Bullet.BP_Bullet_C" (Transformation|GetWorldTransform (Variables|Default|GetArrow)) "Undefined" 0 0))