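; Level-exit portal for the coin game that stays hidden and non-collidable until enough coins are collected, then opens a set level on overlap.
; GetCoin updates the counter text and, at the target total, swaps it for a Clear display, enables the portal and calls ClearMessage on linked BP_Coin2 actors.
; Coins link by matching their PortalTag to the portal's actor tags.
; EventCoinOverlap offers an alternative unlock by checking linked coins' visibility.
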(event OnComponentBeginOverlap(Portal)
  (params (OverlappedComponent :type Primitive%20Component%20Object%20Reference) (OtherActor :type Actor%20Object%20Reference) (OtherComp :type Primitive%20Component%20Object%20Reference) (OtherBodyIndex :type Integer) (bFromSweep :type Boolean) (SweepResult :type Hit%20Result%20Structure%20%28by%20ref%29))
  (Game|OpenLevel(byName) (Variables|Default|GetLevelName)))

(event EventBeginPlay
  (bind _portal (Variables|Default|GetPortal))
  (Rendering|SetVisibility _portal false false)
  (Collision|SetCollisionEnabled _portal "NoCollision")
  (Rendering|Components|TextRender|SetText (Variables|Default|GetCount1) (Utilities|Text|ToText(String) (Utilities|String|Append "/" (Utilities|String|ToString(Integer) (Variables|Default|Get전체코인))))))

(event EventGetCoin
  (bind _portal (Variables|Default|GetPortal))
  (bind _output_get (Variables|Default|Set먹은%20코인 (+ (Variables|Default|Get먹은%20코인) 1)))
  (Rendering|Components|TextRender|SetText (Variables|Default|GetCount) (Utilities|Text|ToText(String) (Utilities|String|Append "COIN " (Utilities|String|ToString(Integer) (Variables|Default|Get먹은%20코인)))))
  (if (>= _output_get (Variables|Default|Get전체코인))
    (Rendering|SetVisibility (Variables|Default|GetCount) false false)
    (Rendering|SetVisibility (Variables|Default|GetClear!) true false)
    (Rendering|SetVisibility _portal true false)
    (Collision|SetCollisionEnabled _portal "QueryAndPhysics")
    (bind _outactors (Actor|GetAllActorsOfClass "/Game/CoinGame/Game2/BP_Coin2.BP_Coin2_C"))
    (for _array_element _outactors
      (if (Actor|ActorHasTag (Variables|/Game/CoinGame/Game2/BP_Coin2.BP_Coin2_C|GetPortalTag _array_element))
        (Class|Clear|Clear(Message) _array_element)))))

(fn ConstructionScript)

(fn EventCoinOverlap
  (bind _portal (Variables|Default|GetPortal))
  (bind _isgetall (CallFunction|IsGetAllCoin))
  (if _isgetall
    (Rendering|SetVisibility _portal true false)
    (Collision|SetCollisionEnabled _portal "QueryAndPhysics")))

(fn IsGetAllCoin
  (bind _outactors (Actor|GetAllActorsOfClass "/Game/CoinGame/Game2/BP_Coin2.BP_Coin2_C"))
  (for _array_element _outactors
    (if (Actor|ActorHasTag (Variables|/Game/CoinGame/Game2/BP_Coin2.BP_Coin2_C|GetPortalTag _array_element))
      (if (Variables|/Script/Engine.SceneComponent|GetbVisible (Variables|/Game/CoinGame/Game2/BP_Coin2.BP_Coin2_C|GetCoin _array_element))
        (return false))))
  (return true))

(fn Count!
  (Rendering|Components|TextRender|SetText (Variables|Default|GetCount) (Utilities|Text|ToText(String) (Utilities|String|Append "COIN " (Utilities|String|ToString(Integer) (Variables|Default|Get먹은%20코인))))))

(fn SetCount
  (Rendering|Components|TextRender|SetText (Variables|Default|GetCount1) (Utilities|Text|ToText(String) (Utilities|String|Append "/" (Utilities|String|ToString(Integer) (Variables|Default|Get전체코인))))))