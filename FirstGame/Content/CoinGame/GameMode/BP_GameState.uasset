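; BP_GameState is the coin game's game state, which tracks elapsed play time and displays it on the HUD.
; Each tick, PrintTime adds delta seconds to a running total and sends a minutes:seconds string to BP_Hud through the first player's controller.
; The STR00 helper floors each value and pads it to two digits with a leading zero.
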(event EventTick
  (params (DeltaSeconds :type Float%20%28single-precision%29))
  (CallFunction|PrintTime DeltaSeconds))

(fn ConstructionScript)

(fn PrintTime
  (params (DeltaSec :type Float%20%28double-precision%29))
  (bind _output_get (Variables|Default|SetTotalSec (+ DeltaSec (Variables|Default|GetTotalSec))))
  (bind _asbp_hud (Utilities|Casting|CastToBP_Hud (HUD|GetHUD (Game|GetPlayerController 0))))
  (Default|SetTimeText _asbp_hud (Utilities|String|Append (CallFunction|STR00 (/ _output_get 6e+01)) ":" (CallFunction|STR00 (Math|Float|%(Float) _output_get 6e+01)))))

(fn STR00
  (params (Num :type Float%20%28double-precision%29))
  (bind _returnvalue (Math|Float|Floor Num))
  (bind _returnvalue_2 (Utilities|String|ToString(Integer) _returnvalue))
  (if (< _returnvalue 10)
    (return (Utilities|String|Append "0" _returnvalue_2))
    (else
      (return _returnvalue_2))))