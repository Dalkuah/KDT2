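; Player state for the coin game, tracking HP, coins, and red, green and black item counts.
; Coin and item add/use functions push counts straight to BP_Hud, except AddBlack, which broadcasts through a dispatcher.
; Damage and heal adjust HP without clamping and broadcast the change.
; BeginPlay broadcasts HP before resetting it to max, then updates the HUD directly; Ragdoll is an empty stub.
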(event EventBeginPlay
  (Default|CallEventDispatcherChange (Variables|Default|GetCurHP) (Variables|Default|GetMaxHP))
  (Variables|Default|SetCurHP (Variables|Default|GetMaxHP))
  (bind _asbp_hud (Utilities|Casting|CastToBP_Hud (HUD|GetHUD (Game|GetPlayerController 0))))
  (Default|SetProgressHP _asbp_hud (Variables|Default|GetCurHP) (Variables|Default|GetMaxHP))
  (Development|PrintString "Begin Play - SetProgressHP" true true "(R=0.000000,G=0.660000,B=1.000000,A=1.000000)" 6e+01))

(fn ConstructionScript)

(fn AddCoin
  (bind _output_get (Variables|Default|SetCoin (+ (Variables|Default|GetCoin) 1)))
  (bind _asbp_hud (Utilities|Casting|CastToBP_Hud (HUD|GetHUD (Game|GetPlayerController 0))))
  (Default|SetCoinText _asbp_hud _output_get))

(fn AddRedItem
  (bind _output_get (Variables|Default|SetRedItem (+ (Variables|Default|GetRedItem) 1)))
  (bind _asbp_hud (Utilities|Casting|CastToBP_Hud (HUD|GetHUD (Game|GetPlayerController 0))))
  (Default|SetRedItemText _asbp_hud _output_get))

(fn UseRedItem
  (bind _output_get (Variables|Default|SetRedItem (+ (Variables|Default|GetRedItem) -1)))
  (bind _asbp_hud (Utilities|Casting|CastToBP_Hud (HUD|GetHUD (Game|GetPlayerController 0))))
  (Default|SetRedItemText _asbp_hud _output_get))

(fn AddGreenItem
  (bind _output_get (Variables|Default|SetGreenItem (+ (Variables|Default|GetGreenItem) 1)))
  (bind _asbp_hud (Utilities|Casting|CastToBP_Hud (HUD|GetHUD (Game|GetPlayerController 0))))
  (Default|SetGreenItemText _asbp_hud _output_get))

(fn UseGreenItem
  (bind _output_get (Variables|Default|SetGreenItem (+ (Variables|Default|GetGreenItem) -1)))
  (bind _asbp_hud (Utilities|Casting|CastToBP_Hud (HUD|GetHUD (Game|GetPlayerController 0))))
  (Default|SetGreenItemText _asbp_hud _output_get))

(fn AddBlackItem
  (bind _output_get (Variables|Default|SetBlackItem (+ (Variables|Default|GetBlackItem) 1)))
  (bind _asbp_hud (Utilities|Casting|CastToBP_Hud (HUD|GetHUD (Game|GetPlayerController 0))))
  (Default|SetBlackItemText _asbp_hud _output_get))

(fn UseBlackItem
  (bind _output_get (Variables|Default|SetBlackItem (+ (Variables|Default|GetBlackItem) -1)))
  (bind _asbp_hud (Utilities|Casting|CastToBP_Hud (HUD|GetHUD (Game|GetPlayerController 0))))
  (Default|SetBlackItemText _asbp_hud _output_get))

(fn AddDamage
  (params (Damage :type Float%20%28double-precision%29))
  (Variables|Default|SetCurHP (- (Variables|Default|GetCurHP) Damage))
  (Default|CallEventDispatcherChange (Variables|Default|GetCurHP) (Variables|Default|GetMaxHP)))

(fn AddHeal
  (params (Heal :type Float%20%28double-precision%29))
  (Variables|Default|SetCurHP (+ (Variables|Default|GetCurHP) Heal))
  (Default|CallEventDispatcherChange (Variables|Default|GetCurHP) (Variables|Default|GetMaxHP)))

(fn Ragdoll)

(fn AddBlack
  (bind _output_get (Variables|Default|SetBlackItem (+ (Variables|Default|GetBlackItem) 1)))
  (Default|CallEventDispatcherChangeBlackItem _output_get))