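; Coin pickup actor that spins and awards a coin to the player state when the third-person character overlaps it.
; A looping timer calls UpdateRotation to rotate the mesh, and pickup disables collision and hides it rather than destroying it.
; BeginPlay also loops over Time-tagged BP_포탈 actors without acting on them.
; CustomEvent hides the coin and pauses a ShowCoin timer, though no such function is defined here.
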(event OnComponentBeginOverlap(Coin)
  (params (OverlappedComponent :type Primitive%20Component%20Object%20Reference) (OtherActor :type Actor%20Object%20Reference) (OtherComp :type Primitive%20Component%20Object%20Reference) (OtherBodyIndex :type Integer) (bFromSweep :type Boolean) (SweepResult :type Hit%20Result%20Structure%20%28by%20ref%29))
  (bind _coin (Variables|Default|GetCoin))
  (bind _asbp_third_person_character (Utilities|Casting|CastToBP_ThirdPersonCharacter OtherActor))
  (bind _asbp_player_state (Utilities|Casting|CastToBP_PlayerState (Variables|/Script/Engine.Pawn|GetPlayerState _asbp_third_person_character)))
  (Default|AddCoin _asbp_player_state)
  (Collision|SetCollisionEnabled _coin "NoCollision")
  (Rendering|SetVisibility _coin false false))

(event Custom|CustomEvent
  (bind _coin (Variables|Default|GetCoin))
  (Class|KismetSystemLibrary|PauseTimer 0 "ShowCoin")
  (Collision|SetCollisionEnabled _coin "NoCollision")
  (Rendering|SetVisibility _coin false false))

(event EventBeginPlay
  (Utilities|Time|SetTimerbyFunctionName 0 "UpdateRotation" 0.01 true)
  (bind _outactors (Actor|GetAllActorsOfClasswithTag "/Game/CoinGame/Practice/BP_포탈.BP_포탈_C" "Time"))
  (for _array_element _outactors
    _))

(fn ConstructionScript)

(fn UpdateRotation
  (Transformation|AddRelativeRotation (Variables|Default|GetCoin) "0.000000,1.000000,0.000000" false false))