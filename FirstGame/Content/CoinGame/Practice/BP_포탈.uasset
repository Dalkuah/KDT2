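; BP_포털 is a level-exit portal for the coin game that opens the level named by LevelName when anything overlaps it.
; Every Tick it compares BP_GameState's TotalSec to MaxTime; once reached, it calls ShowPortal(true) and ClearMessage on every BP_코인, repeating each frame.
; ShowPortal's flag is inverted: true hides the portal and disables collision, so it starts visible and active, then disappears at the time limit.
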(event OnComponentBeginOverlap(Portal)
  (params (OverlappedComponent :type Primitive%20Component%20Object%20Reference) (OtherActor :type Actor%20Object%20Reference) (OtherComp :type Primitive%20Component%20Object%20Reference) (OtherBodyIndex :type Integer) (bFromSweep :type Boolean) (SweepResult :type Hit%20Result%20Structure%20%28by%20ref%29))
  (Game|OpenLevel(byName) (Variables|Default|GetLevel%20Name)))

(event EventBeginPlay
  (CallFunction|ShowPortal false))

(event EventTick
  (params (DeltaSeconds :type Float%20%28single-precision%29))
  (CallFunction|CheckPortal))

(fn ConstructionScript)

(fn ShowPortal
  (params (ShowPortal :type Boolean))
  (bind _portal (Variables|Default|GetPortal))
  (if ShowPortal
    (Rendering|SetVisibility _portal false false)
    (Collision|SetCollisionEnabled _portal "NoCollision")
    (else
      (Rendering|SetVisibility _portal true false)
      (Collision|SetCollisionEnabled _portal "QueryAndPhysics"))))

(fn CheckPortal
  (bind _asbp_game_state (Utilities|Casting|CastToBP_GameState (Game|GetGameState)))
  (if (>= (Variables|/Game/CoinGame/GameMode/BP_GameState.BP_GameState_C|GetTotalSec _asbp_game_state) (Variables|Default|GetMaxTime))
    (CallFunction|ShowPortal true)
    (bind _outactors (Actor|GetAllActorsOfClass "/Game/CoinGame/Practice/BP_코인.BP_코인_C"))
    (for _array_element _outactors
      (Class|Clear|Clear(Message) _array_element))))