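; BP_TimeCoin is a spinning coin pickup that adds a coin to the overlapping third-person character's player state.
; On pickup it disables collision, plays a vertical timeline animation, spawns an effect and hides, then a timer restores it shortly after.
; The Clear event pauses that respawn and hides the coin.
; BeginPlay starts the looping rotation timer and caches a "Time"-tagged BP_TimePortal2, which these graphs never use.
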(event OnComponentBeginOverlap(Coin)
  (params (OverlappedComponent :type Primitive%20Component%20Object%20Reference) (OtherActor :type Actor%20Object%20Reference) (OtherComp :type Primitive%20Component%20Object%20Reference) (OtherBodyIndex :type Integer) (bFromSweep :type Boolean) (SweepResult :type Hit%20Result%20Structure%20%28by%20ref%29))
  (bind _asbp_third_person_character (Utilities|Casting|CastToBP_ThirdPersonCharacter OtherActor))
  (bind _asbp_player_state (Utilities|Casting|CastToBP_PlayerState (Variables|/Script/Engine.Pawn|GetPlayerState _asbp_third_person_character)))
  (Default|AddCoin _asbp_player_state)
  (Collision|SetCollisionEnabled (Variables|Default|GetCoin) "NoCollision")
  (bind _새_트랙_0 (Timeline|Good PlayFromStart)
    (:Update
      (Transformation|SetRelativeLocation (Variables|Default|GetCoin) (Math|Vector|MakeVector 0.0 0.0 (* _새_트랙_0 1e+02)) false false))
    (:Finished
      (Niagara|SpawnSystematLocation "/Game/CoinGame/Good.Good" (Transformation|GetActorLocation))
      (CallFunction|Hidden)
      (Utilities|Time|SetTimerbyFunctionName 0 "ShowCoin" 3.0))))

(event EventBeginPlay
  (Utilities|Time|SetTimerbyFunctionName 0 "UpdateRotation" 0.01 true)
  (bind _outactors (Actor|GetAllActorsOfClasswithTag "/Game/CoinGame/TimeGame/BP_TimePortal2.BP_TimePortal2_C" "Time"))
  (for _array_element _outactors
    (Variables|Default|Setportal _array_element)))

(event EventClear
  (Class|KismetSystemLibrary|PauseTimer 0 "ShowCoin")
  (Collision|SetCollisionEnabled (Variables|Default|GetCoin) "NoCollision")
  (CallFunction|Hidden))

(fn ConstructionScript)

(fn UpdateRotation
  (Transformation|AddRelativeRotation (Variables|Default|GetCoin) "0.000000,1.000000,0.000000" false false))

(fn ShowCoin
  (bind _coin (Variables|Default|GetCoin))
  (Rendering|SetVisibility _coin true false)
  (Collision|SetCollisionEnabled _coin "QueryAndPhysics"))

(fn Hidden
  (Rendering|SetVisibility (Variables|Default|GetCoin) false false))