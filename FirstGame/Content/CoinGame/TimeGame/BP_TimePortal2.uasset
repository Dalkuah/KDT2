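; Level-exit portal for the timed coin game, hidden and non-colliding until time runs out, that opens LevelName on overlap.
; Every Tick polls BP_GameState's TotalSec against MaxTime; once reached, it swaps the counter texts for TimeOver, enables the portal and calls ClearMessage on every BP_TimeCoin, repeating each frame.
; GetCoin increments the displayed coin count, which does not gate the portal.
; PrintTime and SetCount are empty stubs.
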(event OnComponentBeginOverlap(Portal)
  (params (OverlappedComponent :type Primitive%20Component%20Object%20Reference) (OtherActor :type Actor%20Object%20Reference) (OtherComp :type Primitive%20Component%20Object%20Reference) (OtherBodyIndex :type Integer) (bFromSweep :type Boolean) (SweepResult :type Hit%20Result%20Structure%20%28by%20ref%29))
  (Game|OpenLevel(byName) (Variables|Default|GetLevelName)))

(event EventBeginPlay
  (CallFunction|ShowPortal false))

(event EventGetCoin
  (Variables|Default|Set먹은%20코인 (+ (Variables|Default|Get먹은%20코인) 1))
  (Rendering|Components|TextRender|SetText (Variables|Default|GetCount) (Utilities|Text|ToText(String) (Utilities|String|Append "COIN " (Utilities|String|ToString(Integer) (Variables|Default|Get먹은%20코인))))))

(event EventTick
  (params (DeltaSeconds :type Float%20%28single-precision%29))
  (CallFunction|PrintTime DeltaSeconds)
  (CallFunction|ClearCheck))

(fn ConstructionScript)

(fn EventCoinOverlap
  (bind _portal (Variables|Default|GetPortal))
  (if (>= (Variables|Default|GetTotalSec) (Variables|Default|GetMaxTime))
    (Rendering|SetVisibility _portal true false)
    (Collision|SetCollisionEnabled _portal "QueryAndPhysics")))

(fn IsGetAllCoin
  (bind _outactors (Actor|GetAllActorsOfClass "/Game/CoinGame/Game1/BP_Coin.BP_Coin_C"))
  (for _array_element _outactors
    (if (Variables|/Script/Engine.SceneComponent|GetbVisible (Variables|/Game/CoinGame/Game1/BP_Coin.BP_Coin_C|GetCoin _array_element))
      (return false)))
  (return true))

(fn Count!
  (Rendering|Components|TextRender|SetText (Variables|Default|GetCount) (Utilities|Text|ToText(String) (Utilities|String|Append "COIN " (Utilities|String|ToString(Integer) (Variables|Default|Get먹은%20코인))))))

(fn SetCount)

(fn STR00
  (params (Num :type Float%20%28double-precision%29))
  (bind _returnvalue (Math|Float|Floor Num))
  (bind _returnvalue_2 (Utilities|String|ToString(Integer) _returnvalue))
  (if (< _returnvalue 10)
    (return (Utilities|String|Append "0" _returnvalue_2))
    (else
      (return _returnvalue_2))))

(fn PrintTime
  (params (Delta%20Seconds :type Float%20%28double-precision%29)))

(fn ShowPortal
  (params (Show :type Boolean))
  (bind _portal (Variables|Default|GetPortal))
  (if Show
    (Rendering|SetVisibility _portal true false)
    (Collision|SetCollisionEnabled _portal "QueryAndPhysics")
    (else
      (Rendering|SetVisibility _portal false false)
      (Collision|SetCollisionEnabled _portal "NoCollision"))))

(fn ClearCheck
  (bind _asbp_game_state (Utilities|Casting|CastToBP_GameState (Game|GetGameState)))
  ;[1 1 1] 클리어
  (if (>= (Variables|/Game/CoinGame/GameMode/BP_GameState.BP_GameState_C|GetTotalSec _asbp_game_state) (Variables|Default|GetMaxTime))
    (Rendering|SetVisibility (Variables|Default|GetCount) false false)
    (Rendering|SetVisibility (Variables|Default|GetTimeOver!) true false)
    (CallFunction|ShowPortal true)
    (bind _outactors (Actor|GetAllActorsOfClass "/Game/CoinGame/TimeGame/BP_TimeCoin.BP_TimeCoin_C"))
    (for _array_element _outactors
      (Class|Clear|Clear(Message) _array_element))))