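; Blueprint that slides its Cube component back and forth along its relative X axis while playing.
; Start and End events toggle IsPlay, which gates the Tick movement.
; Each Tick offsets the cube by Speed scaled by delta time and flips the MoveRight flag when it passes either hard-coded limit.
; TotalSec accumulates play time but does not drive the motion.
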(event EventTick
  (params (DeltaSeconds :type Float%20%28single-precision%29))
  (bind _cube (Variables|Default|GetCube))
  (bind _cube_2 (Variables|Default|GetCube))
  (if (Variables|Default|GetIsPlay)
    (Variables|Default|SetTotalSec (+ DeltaSeconds (Variables|Default|GetTotalSec)))
    (if (Variables|Default|GetMoveRight)
      (Transformation|AddRelativeLocation _cube_2 (Math|Vector|MakeVector (* DeltaSeconds (Variables|Default|GetSpeed)) 0.0 0.0) false false)
      (if (> (.x (.location (Transformation|GetRelativeTransform _cube_2))) 5e+02)
        (Variables|Default|SetMoveRight false))
      (else
        (Transformation|AddRelativeLocation _cube (Math|Vector|MakeVector (* (* DeltaSeconds (Variables|Default|GetSpeed)) -1.0) 0.0 0.0) false false)
        (if (< (.x (.location (Transformation|GetRelativeTransform _cube))) 0.0)
          (Variables|Default|SetMoveRight true))))))

(event EventEnd
  (Variables|Default|SetIsPlay false))

(event EventStart
  (Variables|Default|SetIsPlay true))

(fn ConstructionScript)