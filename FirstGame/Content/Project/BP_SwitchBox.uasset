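; BP_SwitchBox is a trigger switch whose Cube starts movers while something overlaps it and stops them when the overlap ends.
; Begin and end overlap send StartMessage and EndMessage to every BP_MoveLeftRight and BP_MoveRect found through GetAllActorsOfClass.
; The same messages also go to entries in its Actors array that implement the BPI_MoveActor interface, with no filter on which actor overlaps.
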(event OnComponentBeginOverlap(Cube)
  (params (OverlappedComponent :type Primitive%20Component%20Object%20Reference) (OtherActor :type Actor%20Object%20Reference) (OtherComp :type Primitive%20Component%20Object%20Reference) (OtherBodyIndex :type Integer) (bFromSweep :type Boolean) (SweepResult :type Hit%20Result%20Structure%20%28by%20ref%29))
  (bind _outactors (Actor|GetAllActorsOfClass "/Game/Project/BP_MoveLeftRight.BP_MoveLeftRight_C"))
  (for _array_element _outactors
    (Class|BPIMoveActor|Start(Message) _array_element))
  (bind _outactors_2 (Actor|GetAllActorsOfClass "/Game/Project/BP_MoveRect.BP_MoveRect_C"))
  (for _array_element_2 _outactors_2
    (Class|BPIMoveActor|Start(Message) _array_element_2))
  (for _array_element_3 (Variables|Default|GetActors)
    (if (Utilities|DoesObjectImplementInterface _array_element_3 "/Game/Project/BPI_MoveActor.BPI_MoveActor_C")
      (Class|BPIMoveActor|Start(Message) _array_element_3))))

(event OnComponentEndOverlap(Cube)
  (params (OverlappedComponent :type Primitive%20Component%20Object%20Reference) (OtherActor :type Actor%20Object%20Reference) (OtherComp :type Primitive%20Component%20Object%20Reference) (OtherBodyIndex :type Integer))
  (bind _outactors (Actor|GetAllActorsOfClass "/Game/Project/BP_MoveLeftRight.BP_MoveLeftRight_C"))
  (for _array_element _outactors
    (Class|BPIMoveActor|End(Message) _array_element))
  (bind _outactors_2 (Actor|GetAllActorsOfClass "/Game/Project/BP_MoveRect.BP_MoveRect_C"))
  (for _array_element_2 _outactors_2
    (Class|BPIMoveActor|End(Message) _array_element_2))
  (for _array_element_3 (Variables|Default|GetActors)
    (if (Utilities|DoesObjectImplementInterface _array_element_3 "/Game/Project/BPI_MoveActor.BPI_MoveActor_C")
      (Class|BPIMoveActor|End(Message) _array_element_3))))

(fn ConstructionScript)