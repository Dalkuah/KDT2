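; Spline mover Blueprint that shuttles its Cube back and forth along a spline between calls to its Start and End events.
; A timeline's value, scaled by spline length, gives the distance used to set the Cube's world location without sweeping.
; When the timeline finishes, it flips IsRight and loops back to play or reverse, repeating until End stops it.
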(event EventEnd
  (bind _spline (Variables|Default|GetSpline))
  (bind _value (Timeline|타임라인 Stop)
    (:Update
      (Transformation|SetWorldLocation (Variables|Default|GetCube) (Spline|GetLocationatDistanceAlongSpline _spline (* _value (Spline|GetSplineLength _spline)) "World") false false))
    (:Finished
      (Variables|Default|SetIsRight (not (Variables|Default|GetIsRight)))
      (if (Variables|Default|GetIsRight)
        (Timeline|타임라인 Play)
        (else
          (Timeline|타임라인 Reverse))))))

(event EventStart
  (bind _spline (Variables|Default|GetSpline))
  (if (Variables|Default|GetIsRight) :!label _label
    (bind _value (Timeline|타임라인 Play)
      (:Update
        (Transformation|SetWorldLocation (Variables|Default|GetCube) (Spline|GetLocationatDistanceAlongSpline _spline (* _value (Spline|GetSplineLength _spline)) "World") false false))
      (:Finished
        (Variables|Default|SetIsRight (not (Variables|Default|GetIsRight)))
        (goto _label)))
    (else
      (Timeline|타임라인 Reverse))))

(fn ConstructionScript)