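; BP_MoveRect is a Blueprint that moves its Sphere component around a square loop in the relative X-Z plane.
; While IsPlay is true, Tick offsets the sphere by Speed times DeltaSeconds along the direction held in the SetMove state.
; Crossing each boundary switches SetMove to the next side, cycling right, up, left and down.
; Start and End events toggle the motion, and TotalSec accumulates the playing time.
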(event EventTick
  (params (DeltaSeconds :type Float%20%28single-precision%29))
  (bind _sphere (Variables|Default|GetSphere))
  (bind _sphere_2 (Variables|Default|GetSphere))
  (bind _sphere_3 (Variables|Default|GetSphere))
  (bind _sphere_4 (Variables|Default|GetSphere))
  (if (Variables|Default|GetIsPlay)
    (Variables|Default|SetTotalSec (+ DeltaSeconds (Variables|Default|GetTotalSec)))
    (switch Utilities|FlowControl|Switch|SwitchonEN_MoveType (Variables|Default|GetSetMove)
      (:NewEnumerator0
        (Transformation|AddRelativeLocation _sphere (Math|Vector|MakeVector (* DeltaSeconds (Variables|Default|GetSpeed)) 0.0 0.0) false false)
        (if (> (.x (.location (Transformation|GetRelativeTransform _sphere))) 5e+02)
          (Variables|Default|SetSetMove "NewEnumerator1")))
      (:NewEnumerator1
        (Transformation|AddRelativeLocation _sphere_4 (Math|Vector|MakeVector 0.0 0.0 (* DeltaSeconds (Variables|Default|GetSpeed))) false false)
        (if (> (.z (.location (Transformation|GetRelativeTransform _sphere_4))) 5e+02)
          (Variables|Default|SetSetMove "NewEnumerator2")))
      (:NewEnumerator2
        (Transformation|AddRelativeLocation _sphere_2 (Math|Vector|MakeVector (* -1.0 (* DeltaSeconds (Variables|Default|GetSpeed))) 0.0 0.0) false false)
        (if (< (.x (.location (Transformation|GetRelativeTransform _sphere_2))) 0.0)
          (Variables|Default|SetSetMove "NewEnumerator3")))
      (:NewEnumerator3
        (Transformation|AddRelativeLocation _sphere_3 (Math|Vector|MakeVector 0.0 0.0 (* (* DeltaSeconds (Variables|Default|GetSpeed)) -1.0)) false false)
        (if (< (.z (.location (Transformation|GetRelativeTransform _sphere_3))) 0.0)
          (Variables|Default|SetSetMove "NewEnumerator0"))))))

(event EventEnd
  (Variables|Default|SetIsPlay false))

(event EventStart
  (Variables|Default|SetIsPlay true))

(fn ConstructionScript)