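; BP_MyPawn is a free-flying pawn driven by axis inputs for movement and look.
; Forward, right and up inputs offset the actor along its own axes by a fixed per-event step, without sweep or delta-time scaling, so movement ignores collision and varies with frame rate.
; Look inputs feed controller yaw and pitch, and the construction script is empty.
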(event Input|AxisEvents|InputAxisMoveForward
  (params (AxisValue :type Float%20%28single-precision%29))
  ;[1 0 0] 전/'후
  (Transformation|AddActorWorldOffset (* (Transformation|GetActorForwardVector) (* AxisValue 3e+01))))

(event Input|AxisEvents|InputAxisMoveRight
  (params (AxisValue :type Float%20%28single-precision%29))
  ;[0.1144 1 0] 좌/우
  (Transformation|AddActorWorldOffset (* (Transformation|GetActorRightVector) (* AxisValue 3e+01))))

(event Input|AxisEvents|InputAxisLookUp
  (params (AxisValue :type Float%20%28single-precision%29))
  ;[0.2247 0 1] 방향
  (Pawn|Input|AddControllerPitchInput AxisValue))

(event Input|AxisEvents|InputAxisLookRight
  (params (AxisValue :type Float%20%28single-precision%29))
  ;[0.2247 0 1] 방향
  (Pawn|Input|AddControllerYawInput AxisValue))

(event Input|AxisEvents|InputAxisMoveUp
  (params (AxisValue :type Float%20%28single-precision%29))
  ;[0 0.02461 1] 상/하
  (Transformation|AddActorWorldOffset (* (Transformation|GetActorUpVector) (* AxisValue 3e+01))))

(fn ConstructionScript)